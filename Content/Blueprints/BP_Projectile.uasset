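; Projectile that damages characters and MyBird actors on hit, or knocks hats off characters.
; Each hit plays a pitch-varied sound, then runs Character and bird checks in sequence.
; Hat-tagged components gain physics, reduced projectile velocity, random spin and an extra sound, while bird-tagged components skip bird damage.
; Both checks can destroy the projectile and spawn hit particles, and the damage range is fixed despite its randomization comment.
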(event Collision|EventHit
  (params (MyComp :type Primitive%20Component%20Object%20Reference) (Other :type Actor%20Object%20Reference) (OtherComp :type Primitive%20Component%20Object%20Reference) (bSelfMoved :type Boolean) (HitLocation :type Vector :default "0, 0, 0") (HitNormal :type Vector :default "0, 0, 0") (NormalImpulse :type Vector :default "0, 0, 0") (Hit :type Hit%20Result%20Structure%20%28by%20ref%29))
  ;[0 1 0] Sound
  (Audio|PlaySoundatLocation "/Game/Sounds/SoundCue_Attentuated.SoundCue_Attentuated" HitLocation "0, 0, 0" (Variables|Default|GetVolumeMultiplier) (Math|Random|RandomFloatinRange 0.8 1.2) 0.0 0 0 0)
  (Utilities|FlowControl|Sequence
    (:then_0
      (Utilities|Casting|CastToCharacter Other
        (:then
          (if (Components|ComponentHasTag OtherComp "Hat")
            ;[1 1 1] Hit Hat
            (Actor|DestroyActor)
            (Physics|SetSimulatePhysics OtherComp true)
            (Physics|SetPhysicsLinearVelocity OtherComp (/ (Variables|/Script/Engine.MovementComponent|GetVelocity (Variables|Default|GetProjectileMovement)) 3.0) false "None")
            (Class|PrimitiveComponent|SetPhysicsAngularVelocityinDegrees OtherComp (Math|Vector|MakeVector (Math|Random|RandomFloatinRange -7.2e+02 7.2e+02) (Math|Random|RandomFloatinRange -7.2e+02 7.2e+02) (Math|Random|RandomFloatinRange -7.2e+02 7.2e+02)) false "None")
            ;[0 1 0] Sound
            (Audio|PlaySoundatLocation "/Game/Sounds/Randomize_01.Randomize_01" HitLocation "0, 0, 0" (* (Variables|Default|GetVolumeMultiplier) 0.25) 1.0 0.0 0 0 0)
            (else
              ;[1 1 1] Hit Character
              (Game|Damage|ApplyDamage Other (Math|Random|RandomFloatinRange 1.1e+02 1.1e+02) (Game|GetInstigatorController) self)
              (Actor|DestroyActor :!label _label)
              (Effects|SpawnEmitteratLocation "/Game/Effects/P_Hit.P_Hit" HitLocation))))
        (:CastFailed
          (goto _label))))
    (:then_1
      (Utilities|Casting|CastToMyBird Other
        (:then
          (if (not (Components|ComponentHasTag OtherComp "bird"))
            (Game|Damage|ApplyDamage Other (Math|Random|RandomFloatinRange 1.1e+02 1.1e+02) (Game|GetInstigatorController) self)
            (Actor|DestroyActor :!label _label_2)
            (Effects|SpawnEmitteratLocation "/Game/Effects/P_Hit.P_Hit" HitLocation)))
        (:CastFailed
          (goto _label_2))))))

(fn ConstructionScript)
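; Bird actor that moves itself every frame while periodically reversing its heading.
; Tick sets the transform from the capsule's location plus normalized Direction, with delta time and Speed added rather than multiplied, and rotation derived from Orientation's X vector.
; A 0.2-second Delay on Tick feeds a FlipFlop that alternates Direction along Y and Orientation along X.
; Movement skips sweeping, and scale is reset to one each frame.
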(event EventBeginPlay)

(event Collision|EventActorBeginOverlap
  (params (OtherActor :type Actor%20Object%20Reference)))

(event EventTick
  (params (DeltaSeconds :type Float%20%28single-precision%29))
  (Transformation|SetActorTransform self (Math|Transform|MakeTransform (+ (+ (Math|Vector|Normalize (Variables|Default|GetDirection)) (+ (Utilities|Time|GetWorldDeltaSeconds) (Variables|Default|Getspeed))) (.Location (Math|Transform|BreakTransform (Transformation|GetWorldTransform (Variables|Collision|GetCapsuleComponent))))) (Math|Conversions|RotationFromXVector (Math|Vector|Normalize (Variables|Default|GetOrientation)))))
  (Utilities|FlowControl|Delay 0.2)
  (Utilities|FlowControl|FlipFlop
    (:A
      (Variables|Default|SetDirection "0,10.000000, 0")
      (Variables|Default|SetOrientation "180.000000, 0, 0"))
    (:B
      (Variables|Default|SetDirection "0,-10.000000, 0")
      (Variables|Default|SetOrientation "-180.000000, 0, 0"))))

(fn ConstructionScript)